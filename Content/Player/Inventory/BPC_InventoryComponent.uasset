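; Player inventory component that stores item structs in an array and broadcasts new, update, remove and sound events.
; AddItem increments the quantity of a name match or appends a new entry.
; RemoveItem decrements the passed struct, removing it at zero, without writing the decrement back to the array.
; Adds and removes run EvaluateItems, which logs contents and requests a sound once the metal-tag count reaches a threshold.
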(event EventBeginPlay)

(fn AddItem
  (params (Item :type S%20Item%20Structure%20%28by%20ref%29))
  (bind (_itemname _itemdescription _tags _quantity _mesh) (Utilities|Struct|BreakS_Item Item))
  (bind (_array_element _array_index) (Utilities|Array|ForEachLoopwithBreak (Variables|Default|GetItems) :!label _label)
    (:LoopBody
      (if (Utilities|Enum|Equal(Enum) (.itemName (Utilities|Struct|BreakS_Item _array_element)) _itemname)
        (Development|PrintText "own this item")
        (bind _result (Math|Integer|IncrementInt (.Quantity (Utilities|Struct|BreakS_Item _array_element)))
          (:%20%20
            (Utilities|Array|SetArrayElem (Variables|Default|GetItems) _array_index (Utilities|Struct|MakeS_Item _itemname _itemdescription _tags _result _mesh))
            (LocalVariables|SetbUpdatedItem true)
            (CallFunction|EvaluateItems)
            (goto _label Break)))
        (else
          (Development|PrintText (Utilities|Text|FormatText "not looking for {n}; looking for {x}" (.itemName (Utilities|Struct|BreakS_Item _array_element)) _itemname)))))
    (:Completed
      (if (LocalVariables|GetbUpdatedItem)
        (Default|CallOnUpdateItem (Utilities|Struct|MakeS_Item _itemname _itemdescription _tags _result _mesh))
        (return)
        (else
          (Development|PrintText "new item")
          (Utilities|Array|AddUnique (Variables|Default|GetItems) Item)
          (Default|CallOnNewItem Item)
          (CallFunction|EvaluateItems)
          (return))))))

(fn RemoveItem
  (params (Item :type S%20Item%20Structure%20%28by%20ref%29))
  (bind _result (Math|Integer|DecrementInt (.Quantity (Utilities|Struct|BreakS_Item Item)))
    (:%20%20
      (if (<= _result 0)
        (Utilities|Array|RemoveItem (Variables|Default|GetItems) Item)
        (Default|CallOnRemoveItem Item)
        (else
          (Default|CallOnUpdateItem Item)))
      (CallFunction|EvaluateItems)
      (return))))

(fn GetItem
  (params (ItemToFind :type S%20Item%20Structure%20%28by%20ref%29))
  (bind _items (Variables|Default|GetItems))
  (bind _returnvalue (Utilities|Array|FindItem _items ItemToFind))
  (bind _output (Utilities|Array|Get(acopy) _items _returnvalue))
  (bind (_itemname _itemdescription _tags _quantity _mesh) (Utilities|Struct|BreakS_Item _output))
  (return _itemname _itemdescription _tags _quantity _mesh))

(fn EvaluateItems
  (for (_array_element _array_index) (Variables|Default|GetItems)
    (Development|PrintText (Utilities|Text|FormatText "#{index}: {item}: x{quan}" _array_index (.itemname _array_element) (.quantity _array_element)))
    (if (Utilities|Array|ContainsItem (GameplayTags|BreakGameplayTagContainer (.tags _array_element)) "(TagName=\"Item.Material.Metal\")")
      (Math|Integer|IncrementInt (LocalVariables|GetMetalCount))))
  (if (>= (LocalVariables|GetMetalCount) 2)
    (Default|CallOnAddSound "NewEnumerator1")
    (else
      (Development|PrintText "no sound evaluatioed"))))