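; Base throwable actor that is launched as a projectile and sticks to whatever it hits.
; Throw adds a ProjectileMovement component at runtime, interpolates speed and gravity from strength, enables box collision and sets a limited lifespan.
; On overlap with anything but the instigator, it removes the movement, attaches to the hit component and plays impact sound and particles.
; Physics-simulating targets receive the stored launch velocity as a velocity-change impulse.
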(event OnComponentBeginOverlap(Box)
  (params (OverlappedComponent :type Primitive%20Component%20Object%20Reference) (OtherActor :type Actor%20Object%20Reference) (OtherComp :type Primitive%20Component%20Object%20Reference) (OtherBodyIndex :type Integer) (bFromSweep :type Boolean) (SweepResult :type Hit%20Result%20Structure%20%28by%20ref%29))
  (bind (_bblockinghit _binitialoverlap _time _distance _location _impactpoint _normal _impactnormal _physmat _hitactor _hitcomponent) (Collision|BreakHitResult SweepResult))
  (if (!= OtherActor (Game|GetInstigator))
    (bind _projectile (Variables|Reference|Getprojectile)
      (:then
        (Components|DestroyComponent _projectile))
      (:else
        _))
    (Collision|SetCollisionEnabled (Variables|Default|GetBox) "QueryAndPhysics")
    (Transformation|AttachComponentToComponent _hitcomponent "None" "KeepWorld" "KeepWorld" "KeepWorld" true)
    (Audio|PlaySoundatLocation 0 (Transformation|GetActorLocation) "0, 0, 0" 1.0 1.0 0.0 0 0 0 0)
    (Effects|SpawnEmitteratLocation (Variables|Default|GetimpactEffect) _location)
    (if (Physics|IsSimulatingPhysics _hitcomponent "None")
      (Physics|AddImpulse _hitcomponent (Variables|Default|Getvelocity) "None" true))))

(event Custom|Throw
  (params (direction :type Vector) (strength :type Float%20%28double-precision%29))
  (bind _returnvalue (AddComponent|AddProjectileMovementComponent))
  (Variables|Reference|Setprojectile _returnvalue)
  (bind _output_get (Variables|/Script/Engine.MovementComponent|SetVelocity (Variables|Reference|Getprojectile) (* direction (Math|Float|Lerp (Variables|Default|GetminSpeed) (Variables|Default|GetmaxSpeed) strength))))
  (Variables|Default|Setvelocity _output_get)
  (Variables|/Script/Engine.ProjectileMovementComponent|SetProjectileGravityScale (Variables|Reference|Getprojectile) (Math|Float|Lerp (Variables|Default|GetmaxGravity) (Variables|Default|GetminGravity) strength))
  (Actor|SetLifeSpan 1e+01)
  (Collision|SetCollisionEnabled (Variables|Default|GetBox) "QueryAndPhysics"))

(event EventBeginPlay
  (Collision|SetCollisionEnabled (Variables|Default|GetBox) "NoCollision"))

(fn ConstructionScript)