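; Character component that handles aiming and throwing a spawned throwable actor.
; Aiming attaches the throwable to a mesh socket, turns the character with controller rotation and accumulates aim time on a looping timer.
; Throwing launches it using a camera line trace for direction and normalized aim time for strength, alongside a montage.
; When the montage ends, aim state resets and any queued aim restarts.
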(event Custom|Aim%20Begin
  (bind _character (Variables|Reference|Getcharacter))
  (bind _charactermovement (Variables|/Script/Engine.Character|GetCharacterMovement _character))
  (if (and (not (Variables|Default|GetisAiming?)) (not (Variables|Default|GetisThrowing?)))
    (Variables|Default|SetisWaitingToThrow? false)
    (Variables|Default|SetisAiming? true)
    ;[0.25 0.25 1] Aim Camera Begin
    (Variables|/Script/Engine.CharacterMovementComponent|SetbOrientRotationToMovement _charactermovement false)
    (Variables|/Script/Engine.CharacterMovementComponent|SetbUseControllerDesiredRotation _charactermovement true)
    (Variables|/Script/Engine.CharacterMovementComponent|SetRotationRate _charactermovement (Variables|MovementSettings|GetaimRotationRate))
    (CallFunction|EquipThrowable)
    (bind _returnvalue (Utilities|Time|SetTimerbyEvent (delegate Custom|Increment%20Aim%20Time) (Variables|Default|GetaimIncrementTime) true))
    (Variables|Reference|SetaimTimerHandle _returnvalue)
    (Default|CallOnAimBegin)
    (else
      (Variables|Default|SetisWaitingToThrow? true))))

(event Custom|Aim%20End
  (bind _character (Variables|Reference|Getcharacter))
  (bind _charactermovement (Variables|/Script/Engine.Character|GetCharacterMovement _character))
  (Variables|Default|SetisAiming? false)
  (Variables|Default|SetisWaitingToThrow? false)
  (Variables|Default|SetaimTime 0.0)
  ;[0.25 0.25 1] Aim Camera End
  (Variables|/Script/Engine.CharacterMovementComponent|SetbOrientRotationToMovement _charactermovement true)
  (Variables|/Script/Engine.CharacterMovementComponent|SetbUseControllerDesiredRotation _charactermovement false)
  (Variables|/Script/Engine.CharacterMovementComponent|SetRotationRate _charactermovement (Variables|MovementSettings|GetinitialRotationRate))
  (Utilities|Time|ClearandInvalidateTimerbyHandle (Variables|Reference|GetaimTimerHandle))
  (Default|CallOnAimEnd)
  (Variables|Reference|Getthrowable
    (:then
      (CallFunction|UnequipThrowable))
    (:else)))

(event Custom|Throw%20Begin
  (if (and (Variables|Default|GetisAiming?) (not (Variables|Default|GetisThrowing?)))
    (Variables|Default|SetisThrowing? true)
    (CallFunction|ReleaseThrowable)
    (Animation|Montage|PlayMontage (Variables|/Script/Engine.Character|GetMesh (Variables|Reference|Getcharacter)) (Variables|ThrowableSettings|GetthrowMontage)
      (:OnCompleted
        _)
      (:OnInterrupted
        _))
    (CallFunction|ThrowEnd)))

(event Custom|Increment%20Aim%20Time
  (bind _output_get (Variables|Default|SetaimTime (+ (Variables|Default|GetaimTime) (Variables|Default|GetaimIncrementTime))))
  (Default|CallOnAimOngoing _output_get (Variables|/Game/Blueprints/Pickups/Throwables/BP_Base_Throwable.BP_Base_Throwable_C|GetmaxAimTime (Variables|Reference|Getthrowable))))

(event Custom|Throw%20End
  (if (Variables|Default|GetisThrowing?)
    (Variables|Default|SetisThrowing? false)
    (CallFunction|AimEnd)
    (if (Variables|Default|GetisWaitingToThrow?)
      (CallFunction|AimBegin))))

(event EventBeginPlay
  (bind _ascharacter (Utilities|Casting|CastToCharacter (Components|GetOwner)))
  (Variables|Reference|Setcharacter _ascharacter)
  (Variables|MovementSettings|SetinitialRotationRate (Variables|/Script/Engine.CharacterMovementComponent|GetRotationRate (Variables|/Script/Engine.Character|GetCharacterMovement (Variables|Reference|Getcharacter)))))

(fn EquipThrowable
  (bind _returnvalue (Game|SpawnActorfromClass (Variables|ThrowableSettings|GetthrowableClass) (Math|Transform|MakeTransform "0, 0, 0" "0, 0, 0" "1.000000,1.000000,1.000000") "Undefined" "MultiplyWithRoot" 0 (Variables|Reference|Getcharacter)))
  (bind _output_get (Variables|Reference|Setthrowable _returnvalue))
  (bind _returnvalue_2 (Transformation|AttachComponentToComponent _output_get (Variables|/Script/Engine.Character|GetMesh (Variables|Reference|Getcharacter)) (Variables|ThrowableSettings|GetthrowableSocketName) "SnapToTarget" "SnapToTarget" "SnapToTarget" true))
  (Variables|/Game/Blueprints/Pickups/Throwables/BP_Base_Throwable.BP_Base_Throwable_C|SetinAimState (Variables|Reference|Getthrowable) _returnvalue_2))

(fn UnequipThrowable
  (Variables|/Game/Blueprints/Pickups/Throwables/BP_Base_Throwable.BP_Base_Throwable_C|SetinAimState (Variables|Reference|Getthrowable) false)
  (bind _throwable (Variables|Reference|Getthrowable)
    (:then
      (Actor|DestroyActor _throwable))
    (:else)))

(fn ReleaseThrowable
  (bind _throwable (Variables|Reference|Getthrowable)
    (:then
      (Transformation|DetachFromActor _throwable "KeepWorld" "KeepWorld" "KeepWorld")
      (bind _direction (CallFunction|CalculateAimDirection))
      (Default|Throw _throwable _direction (Math|Float|Clamp(Float) (Math|Float|NormalizetoRange (Variables|Default|GetaimTime) 0.0 (Variables|/Game/Blueprints/Pickups/Throwables/BP_Base_Throwable.BP_Base_Throwable_C|GetmaxAimTime (Variables|Reference|Getthrowable)))))
      (Variables|Reference|Setthrowable 0))
    (:else)))

(fn CalculateAimDirection
  (bind _character (Variables|Reference|Getcharacter))
  (bind _returnvalue (Actor|GetComponentbyClass _character "/Script/Engine.CameraComponent"))
  (bind _returnvalue_2 (Transformation|GetWorldLocation _returnvalue))
  (bind (_outhit _returnvalue_3) (Collision|LineTraceByChannel _returnvalue_2 (+ (* (Math|Vector|GetForwardVector _returnvalue) 1e+04) _returnvalue_2) "TraceTypeQuery1" false 0 "Persistent"))
  (bind _throwable (Variables|Reference|Getthrowable)
    (:then
      (return (Math|Vector|GetUnitDirection(Vector) (Transformation|GetActorLocation _throwable) (select _returnvalue_3 (.TraceEnd (Collision|BreakHitResult _outhit)) (.Location (Collision|BreakHitResult _outhit))))))
    (:else)))