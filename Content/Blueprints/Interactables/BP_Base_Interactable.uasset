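; BP_Base_Interactable is a base Blueprint for objects that can be interacted with, holding the data that describes an interaction.
; Getter functions expose the prompt, interaction type, hold duration and tap count, plus the world location of an InteractionLocation component.
; It contains no interaction logic of its own, as the event graph and construction script are empty.
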(event EventBeginPlay)

(event Collision|EventActorBeginOverlap
  (params (OtherActor :type Actor%20Object%20Reference)))

(event EventTick
  (params (DeltaSeconds :type Float%20%28single-precision%29)))

(fn ConstructionScript)

(fn GetHoldDuration
  (return (Variables|Default|GetholdDuration)))

(fn GetInteractionLocation
  (return (Transformation|GetWorldLocation (Variables|Default|GetInteractionLocation))))

(fn GetInteractionPrompt
  (return (Variables|Default|Getprompt)))

(fn GetInteractionType
  (return (Variables|Default|GetinteractionType)))

(fn GetTapCount
  (return (Variables|Default|GettapAmount)))