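; Character component that lets the owner interact with nearby actors implementing BPI_Interact through IA_Interact.
; Capsule overlaps maintain an in-range list, whose first entry is the active interactable.
; A runtime-created screen-space widget component shows that interactable's W_InteractionPrompt at its interaction location, falling back to actor location.
; Press interacts immediately, Tap counts presses, and Hold tracks elapsed input time through event dispatchers, with both updating prompt progress.
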(event Custom|Handle%20Capsule%20Overlap%20Begin
  (params (OverlappedComponent :type Primitive%20Component%20Object%20Reference) (OtherActor :type Actor%20Object%20Reference) (OtherComp :type Primitive%20Component%20Object%20Reference) (OtherBodyIndex :type Integer) (bFromSweep :type Boolean) (SweepResult :type Hit%20Result%20Structure%20%28by%20ref%29))
  ;[0.25 0.25 1] Handle the functionality when a character that implements this component overlaps with an interactable.
  (if (Utilities|DoesObjectImplementInterface OtherActor "/Game/Player/Inventory/BPI_Interact.BPI_Interact_C") ; Did we overlap with something\nthat can be interacted with?
    (Utilities|Array|AddUnique (Variables|Default|GetinteractablesInRange) OtherActor)
    (CallFunction|RenderInteractionWidget)))

(event Custom|Interact%20With%20Active%20Interactable
  ;[0.25 0.25 1] Call the Interact function in BPI_Interaction.
  (Utilities|IsValid (CallFunction|GetActiveInteractable)
    (:Is%20Valid
      (Class|BPIInteract|Interact(Message) (CallFunction|GetActiveInteractable) (Components|GetOwner))
      (CallFunction|RenderInteractionWidget)
      (CallFunction|ResetInteractionState))))

(event Custom|Interact%20Begin
  (bind _activeinteractable (CallFunction|GetActiveInteractable))
  (Utilities|IsValid _activeinteractable
    (:Is%20Valid
      (bind _interactiontype (Class|BPIInteract|GetInteractionType(Message) _activeinteractable))
      (switch Utilities|FlowControl|Switch|SwitchonE_InteractionType _interactiontype
        (:NewEnumerator0
          (CallFunction|InteractwithActiveInteractable))
        (:NewEnumerator1
          (EventDispatchers|BindEventtoOnInteractOngoing (EventDispatchers|CreateEvent :!event Custom|Interact%20Hold%20Ongoing))
          (EventDispatchers|BindEventtoOnInteractEnded (delegate Custom|Reset%20Widget%20Progress%20to%200)))
        (:NewEnumerator2
          (CallFunction|InteractTap))))))

(event Custom|Handle%20Capsule%20Overlap%20End
  (params (OverlappedComponent :type Primitive%20Component%20Object%20Reference) (OtherActor :type Actor%20Object%20Reference) (OtherComp :type Primitive%20Component%20Object%20Reference) (OtherBodyIndex :type Integer))
  ;[0.25 0.25 1] Handle the functionality when a character that implements this component overlaps with an interactable.
  (if (Utilities|DoesObjectImplementInterface OtherActor "/Game/Player/Inventory/BPI_Interact.BPI_Interact_C") ; Did we overlap with something\nthat can be interacted with?
    (if (== (CallFunction|GetActiveInteractable) OtherActor) ; Did we leave the range of\nthe focused interactable?
      (CallFunction|ResetInteractionState))
    (Utilities|Array|RemoveItem (Variables|Default|GetinteractablesInRange) (CallFunction|GetActiveInteractable))
    (CallFunction|RenderInteractionWidget)))

(event Custom|Interact%20Hold%20Ongoing
  (params (elapsedSeconds :type Float%20%28double-precision%29))
  (bind _activeinteractable (CallFunction|GetActiveInteractable))
  (Utilities|IsValid _activeinteractable
    (:Is%20Valid
      (bind _duration (Class|BPIInteract|GetHoldDuration(Message) _activeinteractable))
      (bind _interactionwidget (Variables|Reference|GetinteractionWidget)
        (:then
          (Default|SetProgressPercent _interactionwidget (/ elapsedSeconds _duration)))
        (:else
          _))
      (if (> elapsedSeconds _duration)
        (CallFunction|InteractwithActiveInteractable)
        (EventDispatchers|UnbindEventfromOnInteractOngoing (delegate Custom|Interact%20Hold%20Ongoing))))))

(event Custom|Interact%20Tap
  (Math|Integer|IncrementInt (Variables|Default|GetcurrentTapCount)
    (:%20%20
      (bind _count (Class|BPIInteract|GetTapCount(Message) (CallFunction|GetActiveInteractable)))
      (if (<= _count 0) ; In case the tap count isn't\nmore than 0, treat like a Press.
        (CallFunction|InteractwithActiveInteractable)
        (else
          (bind _interactionwidget (Variables|Reference|GetinteractionWidget)
            (:then
              (Default|SetProgressPercent _interactionwidget (/ (Variables|Default|GetcurrentTapCount) _count))
              (if (>= (Variables|Default|GetcurrentTapCount) _count) ; Did we reach the number\nof taps needed?
                (CallFunction|InteractwithActiveInteractable)))
            (:else)))))))

(event Custom|Reset%20Widget%20Progress%20to%200
  (bind _interactionwidget (Variables|Reference|GetinteractionWidget)
    (:then
      (Default|SetProgressPercent _interactionwidget 0.0)
      (EventDispatchers|UnbindEventfromOnInteractEnded (delegate Custom|Reset%20Widget%20Progress%20to%200)))
    (:else)))

(event Input|EnhancedActionEvents|EnhancedInputActionIA_Interact
  (params (ActionValue :type Boolean) (ElapsedSeconds :type Float%20%28double-precision%29) (TriggeredSeconds :type Float%20%28double-precision%29) (InputAction :type Input%20Action%20Object%20Reference :default "/Game/Input/Actions/IA_Interact.IA_Interact"))
  ;[0.25 0.25 1] Handle what happens when the player uses the interact key on an interactable or cancels their input.
  (:Started
    (CallFunction|InteractBegin))
  (:Ongoing
    (Default|CallOnInteractOngoing ElapsedSeconds))
  (:Canceled
    (EventDispatchers|UnbindallEventsfromOnInteractOngoing :!label _label)
    (Default|CallOnInteractEnded))
  (:Completed
    (goto _label)))

(event EventBeginPlay
  (bind _ascharacter (Utilities|Casting|CastToCharacter (Components|GetOwner)))
  (Variables|Reference|Setcharacter _ascharacter)
  (Collision|AssignOnComponentBeginOverlap (Variables|/Script/Engine.Character|GetCapsuleComponent (Variables|Reference|Getcharacter)) (EventDispatchers|CreateEvent :!event Custom|Handle%20Capsule%20Overlap%20Begin))
  (Collision|AssignOnComponentEndOverlap (Variables|/Script/Engine.Character|GetCapsuleComponent (Variables|Reference|Getcharacter)) (EventDispatchers|CreateEvent :!event Custom|Handle%20Capsule%20Overlap%20End))
  (bind _returnvalue (Game|AddComponentbyClass (Components|GetOwner) "/Script/UMG.WidgetComponent" true))
  (bind _output_get (Variables|Reference|SetinteractionWidgetComponent _returnvalue))
  (Class|WidgetComponent|SetWidgetSpace _output_get "Screen")
  (Class|WidgetComponent|SetDrawSize _output_get "(X=250.000000,Y=30.000000)"))

(fn RenderInteractionWidget
  (bind _activeinteractable (CallFunction|GetActiveInteractable))
  (Utilities|IsValid _activeinteractable
    (:Is%20Valid
      (bind _interactiontype (Class|BPIInteract|GetInteractionType(Message) _activeinteractable))
      (bind _prompt (Class|BPIInteract|GetInteractionPrompt(Message) _activeinteractable))
      (bind _returnvalue (UserInterface|CreateWidget "/Game/Widgets/W_InteractionPrompt.W_InteractionPrompt_C" 0 _interactiontype _prompt))
      (Variables|Reference|SetinteractionWidget _returnvalue)
      (UserInterface|SetWidget (Variables|Reference|GetinteractionWidgetComponent) _returnvalue)
      (Transformation|SetWorldLocation (Variables|Reference|GetinteractionWidgetComponent) (CallFunction|GetActiveInteractableLocation) false false))
    (:Is%20Not%20Valid
      (UserInterface|SetWidget (Variables|Reference|GetinteractionWidgetComponent) 0) ; If there's no interactable in range,\nset an empty widget to hide and clear.
    )))

(fn GetActiveInteractable
  (return (Utilities|Array|Get(acopy) (Variables|Default|GetinteractablesInRange))))

(fn ResetInteractionState
  (EventDispatchers|UnbindEventfromOnInteractOngoing (EventDispatchers|CreateEvent :!event Custom|Interact%20Hold%20Ongoing))
  (Variables|Default|SetcurrentTapCount 0))

(fn GetActiveInteractableLocation
  (bind _activeinteractable (CallFunction|GetActiveInteractable))
  (Utilities|IsValid _activeinteractable
    (:Is%20Valid
      (bind _location (Class|BPIInteract|GetInteractionLocation(Message) _activeinteractable))
      (return (Math|Vector|SelectVector (Transformation|GetActorLocation _activeinteractable) _location (Math|Vector|VectorIsZero _location))))))