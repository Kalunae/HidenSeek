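; Base table hiding spot that the player can interact with to hide under and leave again.
; On BeginPlay it hands its player and exit positions to the BPCHidingComponent.
; Interact checks the component's occupied state to begin or end hiding, disabling the table's collision on entry without re-enabling it here.
; The interaction prompt switches between Hide and Unhide from the same state.
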(event EventBeginPlay
  (|CallParentFunction)
  (Variables|/Game/Blueprints/Interactables/HidingSpots/BPC_HidingComponent.BPC_HidingComponent_C|SethidingSpotPosition (Variables|Default|GetBPC_HidingComponent) (Variables|Default|GetPlayerPosition))
  (Variables|/Game/Blueprints/Interactables/HidingSpots/BPC_HidingComponent.BPC_HidingComponent_C|SetexitSpotPosition (Variables|Default|GetBPC_HidingComponent) (Variables|Default|GetExitPosition)))

(event Collision|EventActorBeginOverlap
  (params (OtherActor :type Actor%20Object%20Reference))
  (|CallParentFunction OtherActor) ; This node is disabled and will not be called.\nDrag off pins to build functionality.
)

(event EventTick
  (params (DeltaSeconds :type Float%20%28single-precision%29))
  (|CallParentFunction DeltaSeconds) ; This node is disabled and will not be called.\nDrag off pins to build functionality.
)

(event EventInteract
  (params (interactor :type Actor%20Object%20Reference))
  (if (not (Variables|/Game/Blueprints/Interactables/HidingSpots/BPC_HidingComponent.BPC_HidingComponent_C|GetisOccupied? (Variables|Default|GetBPC_HidingComponent)))
    (Default|HidingBegin (Variables|Default|GetBPC_HidingComponent) interactor)
    (Development|PrintText "Player is hiding under the table.")
    (Collision|SetCollisionEnabled (Variables|Default|GetCollision) "NoCollision")
    (else
      (Default|HidingEnd (Variables|Default|GetBPC_HidingComponent))
      (Development|PrintText "Player left the table."))))

(fn ConstructionScript
  (|CallParentFunction))

(fn GetInteractionPrompt
  (return (select (Variables|/Game/Blueprints/Interactables/HidingSpots/BPC_HidingComponent.BPC_HidingComponent_C|GetisOccupied? (Variables|Default|GetBPC_HidingComponent)) "Unhide" "Hide")))