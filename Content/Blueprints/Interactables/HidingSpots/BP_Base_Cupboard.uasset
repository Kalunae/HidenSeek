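; Base cupboard hiding spot that the player interacts with to hide or leave.
; On BeginPlay it passes its hide and exit positions to BPCHidingComponent, whose occupied state selects the action and the Hide/Unhide prompt.
; Hiding disables Collision and plays a timeline that rotates both doors in mirrored yaw; leaving reverses it, each with its own sound.
; Collision is not re-enabled in this graph.
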(event EventBeginPlay
  (|CallParentFunction)
  (Variables|/Game/Blueprints/Interactables/HidingSpots/BPC_HidingComponent.BPC_HidingComponent_C|SethidingSpotPosition (Variables|Default|GetBPC_HidingComponent) (Variables|Default|GetPlayerPosition))
  (Variables|/Game/Blueprints/Interactables/HidingSpots/BPC_HidingComponent.BPC_HidingComponent_C|SetexitSpotPosition (Variables|Default|GetBPC_HidingComponent) (Variables|Default|GetExitPosition)))

(event Collision|EventActorBeginOverlap
  (params (OtherActor :type Actor%20Object%20Reference))
  (|CallParentFunction OtherActor) ; This node is disabled and will not be called.\nDrag off pins to build functionality.
)

(event EventTick
  (params (DeltaSeconds :type Float%20%28single-precision%29))
  (|CallParentFunction DeltaSeconds) ; This node is disabled and will not be called.\nDrag off pins to build functionality.
)

(event EventInteract
  (params (interactor :type Actor%20Object%20Reference))
  (if (not (Variables|/Game/Blueprints/Interactables/HidingSpots/BPC_HidingComponent.BPC_HidingComponent_C|GetisOccupied? (Variables|Default|GetBPC_HidingComponent)))
    (Default|HidingBegin (Variables|Default|GetBPC_HidingComponent) interactor)
    (Development|PrintText "Player is hiding in the cupboard.")
    (Collision|SetCollisionEnabled (Variables|Default|GetCollision) "NoCollision")
    (Audio|PlaySoundatLocation "/Game/Victorian_House/Audio/Cues/Cue_CloseDoor_01.Cue_CloseDoor_01" (Transformation|GetActorLocation) "0, 0, 0" 1.0 1.0 0.0 0 0 0 0)
    (bind _z_rotation (Timeline|Timeline_Door PlayFromStart)
      (:Update
        (Transformation|SetRelativeRotation (Variables|Default|GetDoor_L) (Math|Rotator|MakeRotator 0.0 0.0 _z_rotation) false false)
        (Transformation|SetRelativeRotation (Variables|Default|GetDoor_R) (Math|Rotator|MakeRotator 0.0 0.0 (* _z_rotation -1.0)) false false)))
    (else
      (Default|HidingEnd (Variables|Default|GetBPC_HidingComponent))
      (Development|PrintText "Player left the cupboard.")
      (Audio|PlaySoundatLocation "/Game/Victorian_House/Audio/Wavs/S_OpenDoor_02.S_OpenDoor_02" (Transformation|GetActorLocation) "0, 0, 0" 1.0 1.0 0.0 0 0 0 0)
      (Timeline|Timeline_Door ReverseFromEnd))))

(fn ConstructionScript
  (|CallParentFunction))

(fn GetInteractionPrompt
  (return (select (Variables|/Game/Blueprints/Interactables/HidingSpots/BPC_HidingComponent.BPC_HidingComponent_C|GetisOccupied? (Variables|Default|GetBPC_HidingComponent)) "Unhide" "Hide")))