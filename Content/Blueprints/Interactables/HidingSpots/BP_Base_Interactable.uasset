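; Base interactable actor that supplies a mesh, an interaction point and interaction settings for items placed in the world.
; The construction script looks up its item row in DT_Items and, when that row's mesh is valid, applies it to InteractableMesh at a scale taken from ItemScale.
; Getter functions expose prompt, interaction type, hold duration, tap count and world interaction location, while the event graph holds no active logic.
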(event EventBeginPlay)

(event Collision|EventActorBeginOverlap
  (params (OtherActor :type Actor%20Object%20Reference)))

(event EventTick
  (params (DeltaSeconds :type Float%20%28single-precision%29)))

(fn ConstructionScript
  (bind _interactablemesh (Variables|Default|GetInteractableMesh))
  (bind _returnvalue (Utilities|GetDataTableRow "/Game/Data/Items/DT_Items.DT_Items" (.rowname (Variables|Default|GetItemInfo)))
    (:then
      (Utilities|IsValid (.mesh _returnvalue)
        (:Is%20Valid
          (Components|StaticMesh|SetStaticMesh _interactablemesh (.mesh _returnvalue))
          (Transformation|SetWorldScale3D _interactablemesh (Math|Conversions|ToVector(Float) (Variables|Default|GetItemScale))))))))

(fn GetHoldDuration
  (return (Variables|Default|GetholdDuration)))

(fn GetInteractionLocation
  (return (Transformation|GetWorldLocation (Variables|Default|GetInteractionLocation))))

(fn GetInteractionPrompt
  (return (Variables|Default|Getprompt)))

(fn GetInteractionType
  (return (Variables|Default|GetinteractionType)))

(fn GetTapCount
  (return (Variables|Default|GettapAmount)))